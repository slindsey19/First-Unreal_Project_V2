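; HOURGLASS is a collectible time pickup actor that grants time through the game HUD when overlapped.
; On overlap it plays a sound at its location, casts the player's HUD to TPGameHUD, calls TimeCollected, then destroys itself.
; Every tick it rotates by a fixed step and plays a timeline whose ORB track drives a local offset to animate the floating motion.
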(event EventBeginPlay)

(event Collision|EventActorBeginOverlap
  (params (OtherActor :type Actor%20Object%20Reference))
  ;[1 1 1] collecting hourglass
  (Audio|PlaySoundatLocation "/Game/StarterContent/Audio/Light02_Cue.Light02_Cue" (Transformation|GetActorLocation) "0, 0, 0" 1.0 1.0 0.0 0 0 0)
  (bind _astpgame_hud (Utilities|Casting|CastToTPGameHUD (HUD|GetHUD (Game|GetPlayerController 0))))
  (bind _output_get (Variables|Default|SetHUD _astpgame_hud))
  (Default|TimeCollected _output_get)
  (Actor|DestroyActor))

(event EventTick
  (params (DeltaSeconds :type Float%20%28single-precision%29))
  ;[1 1 1] actor rotation
  (Transformation|AddActorLocalRotation "0,3.000000, 0" false false)
  (bind _orb (Timeline|Timeline_0 Play)
    (:Update
      (Transformation|AddActorLocalOffset _orb false false))))

(fn ConstructionScript)