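; HUD Blueprint for the TP game that draws a countdown timer and score on screen and also holds the game state.
; BeginPlay calls StartGame, which resets score, key and game-over flags, sets the time and starts a looping one-second timer.
; Each tick of that timer decrements the time, setting game over and clearing itself when time runs out.
; CoinCollected increments score, and TimeCollected extends time through a by-reference Add 10 macro.
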(event Custom|Timer
  ;[1 0 0.001624] Timer - Decrements timer by 1 and checks for game over
  (bind _result (Math|Integer|DecrementInt (Variables|Default|Gettime))
    (:%20%20
      (if (<= _result 0)
        (Variables|Default|Setgameover true)
        (Utilities|Time|ClearTimerbyFunctionName 0 "Timer")))))

(event EventBeginPlay
  (Utilities|StartGame))

(event Collision|EventActorBeginOverlap
  (params (OtherActor :type Actor%20Object%20Reference)))

(event EventTick
  (params (DeltaSeconds :type Float%20%28single-precision%29)))

(event EventDrawHUD
  (params (SizeX :type Integer) (SizeY :type Integer))
  (HUD|DrawText (Utilities|String|ToString(Integer) (Variables|Default|Gettime)) "(R=0,G=0,B=0,A=1)" 1e+01 1e+01 "/Game/Fonts/Windsong_Font.Windsong_Font" 3.0 false)
  (HUD|DrawText (Utilities|String|ToString(Integer) (Variables|Default|Getscore)) "(R=0,G=0,B=0,A=1)" 5e+02 1e+01 0 3.0 false))

(fn ConstructionScript)

(fn CoinCollected
  (Math|Integer|IncrementInt (Variables|Default|Getscore)))

(fn TimeCollected
  (Utilities|Add10 (Variables|Default|Gettime)))